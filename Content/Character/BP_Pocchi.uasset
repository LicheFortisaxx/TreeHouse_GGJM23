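; Player character Pocchi for a platformer, with walk and sprint speeds, multi-jump, wall slide and wall jump.
; While falling, a per-tick capsule trace detects walls, turns Pocchi toward them and lowers gravity for the slide, enabling JumpCheck's launch-based wall jump.
; Landing resets jumps, bounces off and destroys BP_Enemy1, and applies fall damage from vertical speed.
; It also creates the HUD, shows the win widget on trigger overlap and opens SuperiorLvl at zero health.
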(event `WallSlideVelocityReset`
  (bind (_returnvalue_x _returnvalue_y) (`KismetMathLibrary.BreakVector` (`self.GetVelocity`)))
  ;[1 0.007655 0] No me convence mucho
  (goto _label :!via `Reset`))

(event `self.ReceiveBeginPlay`
  (bind _returnvalue (`|CreateWidget` "/Game/Character/W_HUD_Pocchi.W_HUD_Pocchi_C"))
  (`UserWidget.AddToViewport` _returnvalue 0)
  ;[0.3479 1 0.3521] Variable para Speed OFFSET 5.
  (set `self.Default walk speed` (`CharacterMovementComponent.MaxWalkSpeed` (`self.CharacterMovement`)))
  (set `self.Default Gravity ` (`CharacterMovementComponent.GravityScale` (`self.CharacterMovement`))))

(event `self.ReceiveTick`
  (params (DeltaSeconds :type "Float (single-precision)"))
  (bind (_returnvalue_x _returnvalue_y _returnvalue_z) (`KismetMathLibrary.BreakVector` (`self.GetVelocity`)))
  (bind _returnvalue (`self.K2_GetActorLocation`))
  (bind (_returnvalue_x_2 _returnvalue_y_2 _returnvalue_z_2) (`KismetMathLibrary.BreakVector` (`self.GetVelocity`)))
  (bind (_returnvalue_x_3 _returnvalue_y_3) (`KismetMathLibrary.BreakVector` (`self.GetVelocity`)))
  (bind (_returnvalue_roll _returnvalue_pitch _returnvalue_yaw) (`KismetMathLibrary.BreakRotator` (`KismetMathLibrary.Conv_VectorToRotator` (`self.Wall Hit Normal`))))
  ;[0.4271 0.1389 0.04145] 7. Reduccion de velocidad al contacto con pared
  (if (`NavMovementComponent.IsFalling` (`self.CharacterMovement`))
    (bind _outhit (`KismetSystemLibrary.CapsuleTraceSingle` _returnvalue _returnvalue 35.0 69.0 "TraceTypeQuery1"))
    (set `self.BeInWallSlide` (`GameplayStatics.BreakHitResult` _outhit))
    (set `self.Wall Hit Normal` (`.Normal` (`GameplayStatics.BreakHitResult` _outhit)))
    (if (`GameplayStatics.BreakHitResult` _outhit)
      ;[0 1 0.1356] Como paso 10
      (set `self.JumpCount` (- (`self.JumpMaxCount`) 1))
      (`self.K2_SetActorRotation` (`KismetMathLibrary.MakeRotator` 0.0 0.0 (+ _returnvalue_yaw 180.0)))
      (if (<= _returnvalue_z_2 0.0)
        (`|ExecutionSequence`
          (:`then_0`
            ;[1 1 1] Slowly wall slide, more reallistic
            (`/Engine/EditorBlueprintResources/StandardMacros.DoOnce` false :!label _label
              (:`Completed`
                (set `MovementComponent.Velocity` (`KismetMathLibrary.MakeVector` _returnvalue_x_3 _returnvalue_y_3) (`self.CharacterMovement`)))))
          (:`then_1`
            (set `CharacterMovementComponent.GravityScale` 0.15 (`self.CharacterMovement`))
            (set `MovementComponent.Velocity` (`KismetMathLibrary.VInterpTo` (`self.GetVelocity`) (`KismetMathLibrary.MakeVector` 0.0 0.0 _returnvalue_z) (`GameplayStatics.GetWorldDeltaSeconds`) (`self.WalkSlideDesaceleration`)) (`self.CharacterMovement`)))))
      (elif true
        (set `CharacterMovementComponent.GravityScale` (`self.Default Gravity `) (`self.CharacterMovement`))
        ;[1 0.03593 0] No me convence mucho x2
        (`self.WallSlideVelocityReset`)))))

(event `self.WinTrigger.OnActorBeginOverlap`
  (params (OverlappedActor :type "Actor Object Reference") (OtherActor :type "Actor Object Reference"))
  (bind _returnvalue (`|CreateWidget` "/Game/Character/W_Win.W_Win_C"))
  (`UserWidget.AddToViewport` _returnvalue 0))

(event `InputAction|Jump`
  (params (Key :type "Key Structure"))
  ;[0.1831 1 0.628] 4. JUMP
  (:`Pressed`
    (`self.Jump_Check`)
    (`GameplayStatics.PlaySound2D` "/Game/Sounds/jump_Cuee.jump_Cuee" 1.0 1.0 0.0 null null))
  (:`Released`
    (`self.StopJumping`)))

(event `InputAxis|Move/Walk Right/Left`
  (params (AxisValue :type "Float (single-precision)"))
  ;[0.1159 0.2264 1] 1. Movement Logic Ch_Pocchi
  (`self.AddMovementInput` (`KismetMathLibrary.GetForwardVector` (`KismetMathLibrary.MakeRotator` 0.0 0.0 (.yaw (`self.GetControlRotation`)))) AxisValue))

(event `self.OnLanded`
  (params (Hit :type "HitResult Structure (by ref)"))
  (bind (_returnvalue_x _returnvalue_y _returnvalue_z) (`KismetMathLibrary.BreakVector` (`self.GetVelocity`)))
  (`|ExecutionSequence`
    (:`then_0`
      (set `self.JumpCount` 0)
      ;[0 0.7292 1] Jump bug Fixed
      (set `self.BeInWallSlide` false)
      (set `self.JumpCount` 0)
      (`self.WallSlideVelocityReset`)
      (set `CharacterMovementComponent.GravityScale` (`self.Default Gravity `) (`self.CharacterMovement`)))
    (:`then_1`
      (bind _asbp_enemy_1 (cast `/Game/Enemy_1/BP_Enemy1` (`.HitActor` (`GameplayStatics.BreakHitResult` Hit))))
      (`|PlayMontage` (`/Game/Enemy_1/BP_Enemy1.Sapria` _asbp_enemy_1) "/Game/Enemy_1/Model_Flor_Sapria/FlorSapia_Anim_Montage.FlorSapia_Anim_Montage" 0.2
        (:`then`
          (`GameplayStatics.PlaySound2D` "/Game/Sounds/boing_sapria_Cuee.boing_sapria_Cuee" 2.5 1.0 0.0 null null)
          (`KismetSystemLibrary.Delay` 0.5)
          (`self.K2_DestroyActor` _asbp_enemy_1)
          (`self.LaunchCharacter` (* (`KismetMathLibrary.Vector_Up`) (`self.BounceHieght`))))))
    (:`then_2`
      ;[1 1 1] Aplicar daño de caida y normalizar vecto
      (`GameplayStatics.ApplyDamage` self (`KismetMathLibrary.FClamp` (`KismetMathLibrary.NormalizeToRange` (`KismetMathLibrary.Abs` _returnvalue_z) 1000.0 1600.0))))))

(event `InputAction|Walk`
  (params (Key :type "Key Structure"))
  ;[0.2763 1 0.5679] 5. Speed Offsets FIAUU
  (:`Pressed`
    (set `CharacterMovementComponent.MaxWalkSpeed` (* (`self.Walk Speed Offset`) (`self.Default walk speed`)) (`self.CharacterMovement`)))
  (:`Released`
    (set `CharacterMovementComponent.MaxWalkSpeed` (`self.Default walk speed`) (`self.CharacterMovement`))))

(event `InputAction|Sprint`
  (params (Key :type "Key Structure"))
  ;[0.2763 1 0.5679] 5. Speed Offsets FIAUU
  (:`Pressed`
    (set `CharacterMovementComponent.MaxWalkSpeed` (* (`self.Speed sprint Offset`) (`self.Default walk speed`)) (`self.CharacterMovement`)))
  (:`Released`
    (set `CharacterMovementComponent.MaxWalkSpeed` (`self.Default walk speed`) (`self.CharacterMovement`))))

(event `self.ReceiveAnyDamage`
  (params (Damage :type "Float (single-precision)") (DamageType :type "DamageType Object Reference") (InstigatedBy :type "Controller Object Reference") (DamageCauser :type "Actor Object Reference"))
  (bind _health (`self.Health`))
  ;[1 1 1] Daño y reinicio de nivel
  (bind _output_get (set `self.Health` (- _health Damage)))
  (`KismetSystemLibrary.PrintString` (`KismetStringLibrary.Conv_DoubleToString` _output_get))
  (if (<= _health 0.0)
    (`GameplayStatics.OpenLevelBySoftObjectPtr` "/Game/Level/SuperiorLvl.SuperiorLvl")))

(fn `Jump_Check`
  (if (`self.BeInWallSlide`)
    ;[0 0 0] Wall Jump (Impulsoms)
    (`self.PlayAnimMontage` "/Game/Character/Pocchi_Air_Montage.Pocchi_Air_Montage")
    (`self.LaunchCharacter` (+ (* (`self.GetActorForwardVector`) (`self.WallJumpForce`)) (0.0 0.0 600.0)) true true)
    (`/Engine/EditorBlueprintResources/StandardMacros.IncrementInt` (`self.JumpCount`))
    (else
      ;[0.7189 0.3382 1] 6.Jump, cuidao al agregar mas Play AnimMontages..
      (if (< (`self.JumpCount`) (`self.JumpMaxCount`))
        (if (`NavMovementComponent.IsFalling` (`self.CharacterMovement`))
          ;[0 0 0] Air jump
          (`self.PlayAnimMontage` "/Game/Character/Pocchi_Air_Montage.Pocchi_Air_Montage")
          (`self.Reset Jump Velocity`)
          (`self.LaunchCharacter` (+ (`self.GetVelocity`) (`KismetMathLibrary.MakeVector` 0.0 0.0 (`self.AirJumpForce`))) true true)
          (`/Engine/EditorBlueprintResources/StandardMacros.IncrementInt` (`self.JumpCount`)
            (:`  `
              (bind _output_get (set `self.LimitJump` (- (`self.LimitJump`) 1)))
              (`KismetSystemLibrary.PrintString` (`KismetStringLibrary.Conv_IntToString` _output_get))))
          (else
            ;[0 0 0] Ground Jump
            (`self.Jump`)
            (`/Engine/EditorBlueprintResources/StandardMacros.IncrementInt` (`self.JumpCount`))))))))

(fn `Reset Jump Velocity`
  (set `MovementComponent.Velocity` (`KismetMathLibrary.MakeVector` (.x (`self.GetVelocity`)) (.y (`self.GetVelocity`))) (`self.CharacterMovement`)))

(fn `UserConstructionScript`)